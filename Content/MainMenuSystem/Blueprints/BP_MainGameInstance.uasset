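; Game instance that acts as the central manager for showing menu widgets: boot, loading, main, options, new/load/save game, pause and quit confirmations.
; Each Show event lazily creates its widget once, caches it and adds it to the viewport.
; Main, pause, boot and loading screens also set UI-only input and cursor visibility.
; The pause menu pauses the game, and Resume restores game-only input.
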(event Custom|Show%20WBP_MainMenu
  (bind _returnvalue (Game|GetPlayerController 0))
  ;[1 1 1] Show WBP_MainMenu
  (Utilities|IsValid (Variables|Widjets|GetMainMenuWBP)
    (:Is%20Valid
      _)
    (:Is%20Not%20Valid
      (bind _returnvalue_2 (UserInterface|CreateWidget "/Game/MainMenuSystem/UI/WBP_MainMenu.WBP_MainMenu_C" _returnvalue))
      (bind _output_get (Variables|Widjets|SetMainMenuWBP _returnvalue_2))))
  (UserInterface|Viewport|AddtoViewport _output_get 0)
  (Input|SetInputModeUIOnly _returnvalue (Variables|Widjets|GetMainMenuWBP) "DoNotLock" false)
  (Variables|/Script/Engine.PlayerController|SetbShowMouseCursor _returnvalue true))

(event Custom|Show%20WBP_LoadGame
  ;[1 1 1] Show WBP_LoadGame
  (Utilities|IsValid (Variables|Widjets|GetLoadGameWBP)
    (:Is%20Valid
      _)
    (:Is%20Not%20Valid
      (bind _returnvalue (UserInterface|CreateWidget "/Game/MainMenuSystem/UI/WBP_LoadGame.WBP_LoadGame_C" (Game|GetPlayerController 0)))
      (bind _output_get (Variables|Widjets|SetLoadGameWBP _returnvalue))))
  (UserInterface|Viewport|AddtoViewport _output_get 0))

(event Custom|Show%20WBP_BootScreen
  (bind _returnvalue (Game|GetPlayerController 0))
  ;[1 1 1] Show WBP_BootScreen
  (Utilities|IsValid (Variables|Widjets|GetBootScreenWBP)
    (:Is%20Valid
      _)
    (:Is%20Not%20Valid
      (bind _returnvalue_2 (UserInterface|CreateWidget "/Game/MainMenuSystem/UI/WBP_BootScreen.WBP_BootScreen_C" _returnvalue))
      (bind _output_get (Variables|Widjets|SetBootScreenWBP _returnvalue_2))))
  (UserInterface|Viewport|AddtoViewport _output_get 0)
  (Input|SetInputModeUIOnly _returnvalue (Variables|Widjets|GetBootScreenWBP) "DoNotLock" false)
  (Variables|/Script/Engine.PlayerController|SetbShowMouseCursor _returnvalue false))

(event Custom|Show%20WBP_PauseMenu
  (bind _returnvalue (Game|GetPlayerController 0))
  ;[1 1 1] Show WBP_PauseMenu
  (Utilities|IsValid (Variables|Widjets|GetPauseMenuWBP)
    (:Is%20Valid
      _)
    (:Is%20Not%20Valid
      (bind _returnvalue_2 (UserInterface|CreateWidget "/Game/MainMenuSystem/UI/WBP_PauseMenu.WBP_PauseMenu_C" _returnvalue))
      (bind _output_get (Variables|Widjets|SetPauseMenuWBP _returnvalue_2))))
  (UserInterface|Viewport|AddtoViewport _output_get 0)
  (Game|SetGamePaused true)
  (Input|SetInputModeUIOnly _returnvalue (Variables|Widjets|GetPauseMenuWBP) "DoNotLock" false)
  (Variables|/Script/Engine.PlayerController|SetbShowMouseCursor _returnvalue true))

(event Custom|Show%20WBP_LoadingScreen
  (bind _returnvalue (Game|GetPlayerController 0))
  ;[1 1 1] Show_WBP_LoadingScreen
  (Utilities|IsValid (Variables|Widjets|GetLoadingScreenWBP)
    (:Is%20Valid
      _)
    (:Is%20Not%20Valid
      (bind _returnvalue_2 (UserInterface|CreateWidget "/Game/MainMenuSystem/UI/WBP_LoadingScreen.WBP_LoadingScreen_C" _returnvalue))
      (bind _output_get (Variables|Widjets|SetLoadingScreenWBP _returnvalue_2))))
  (UserInterface|Viewport|AddtoViewport _output_get 0)
  (Input|SetInputModeUIOnly _returnvalue (Variables|Widjets|GetLoadingScreenWBP) "DoNotLock" false)
  (Variables|/Script/Engine.PlayerController|SetbShowMouseCursor _returnvalue false))

(event Custom|Show%20WBP_QuitGame
  ;[1 1 1] Show WBP_QuitGame
  (Utilities|IsValid (Variables|Widjets|GetQuitGameWBP)
    (:Is%20Valid
      _)
    (:Is%20Not%20Valid
      (bind _returnvalue (UserInterface|CreateWidget "/Game/MainMenuSystem/UI/WBP_QuitGameQuestion.WBP_QuitGameQuestion_C" (Game|GetPlayerController 0)))
      (bind _output_get (Variables|Widjets|SetQuitGameWBP _returnvalue))))
  (UserInterface|Viewport|AddtoViewport _output_get 0))

(event Custom|Pause%20Menu%20Resume
  (bind _returnvalue (Game|GetPlayerController 0))
  ;[1 1 1] Pause Menu Resume
  (Widget|RemovefromParent (Variables|Widjets|GetPauseMenuWBP))
  (Game|SetGamePaused false)
  (Input|SetInputModeGameOnly _returnvalue false)
  (Variables|/Script/Engine.PlayerController|SetbShowMouseCursor _returnvalue false))

(event Custom|Show%20WBP_OptionsMenu
  ;[1 1 1] Show WBP_OptionsMenu
  (Utilities|IsValid (Variables|Widjets|GetOptionsMenuWBP)
    (:Is%20Valid
      _)
    (:Is%20Not%20Valid
      (bind _returnvalue (UserInterface|CreateWidget "/Game/MainMenuSystem/UI/Options/WBP_OptionsMenu.WBP_OptionsMenu_C" (Game|GetPlayerController 0)))
      (bind _output_get (Variables|Widjets|SetOptionsMenuWBP _returnvalue))))
  (UserInterface|Viewport|AddtoViewport _output_get 0))

(event Custom|Show%20WBP_QuitToMainMenu
  ;[1 1 1] Show WBP_QuitToMainMenu
  (Utilities|IsValid (Variables|Widjets|GetPauseMenuQuitToMainMenu)
    (:Is%20Valid
      _)
    (:Is%20Not%20Valid
      (bind _returnvalue (UserInterface|CreateWidget "/Game/MainMenuSystem/UI/WBP_QuitToMainMenuQuestion.WBP_QuitToMainMenuQuestion_C" (Game|GetPlayerController 0)))
      (bind _output_get (Variables|Widjets|SetPauseMenuQuitToMainMenu _returnvalue))))
  (UserInterface|Viewport|AddtoViewport _output_get 0)
  (Widget|RemovefromParent (Variables|Widjets|GetPauseMenuWBP)))

(event Custom|Show%20WBP_NewGame
  ;[1 1 1] Show WBP_NewGame
  (Utilities|IsValid (Variables|Widjets|GetNewGameWBP)
    (:Is%20Valid
      _)
    (:Is%20Not%20Valid
      (bind _returnvalue (UserInterface|CreateWidget "/Game/MainMenuSystem/UI/WBP_NewGame.WBP_NewGame_C" (Game|GetPlayerController 0)))
      (bind _output_get (Variables|Widjets|SetNewGameWBP _returnvalue))))
  (UserInterface|Viewport|AddtoViewport _output_get 0))

(event Custom|Show%20WBP_SaveGame
  ;[1 1 1] Show WBP_SaveGame
  (Utilities|IsValid (Variables|Widjets|GetSaveGameWBP)
    (:Is%20Valid
      _)
    (:Is%20Not%20Valid
      (bind _returnvalue (UserInterface|CreateWidget "/Game/MainMenuSystem/UI/WBP_SaveGame.WBP_SaveGame_C" (Game|GetPlayerController 0)))
      (bind _output_get (Variables|Widjets|SetSaveGameWBP _returnvalue))))
  (UserInterface|Viewport|AddtoViewport _output_get 0))