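; Main menu player controller that restores saved audio and mouse settings on BeginPlay.
; It sets SM_Master as the base mix, then applies volumes from the SaveAudio slot as class overrides for Master, Music, SFX and Voice.
; Sensitivity and inversion from SaveMouseSettings are copied onto the player's BP_ThirdPersonCharacter.
; A missing slot only creates a BP_SaveGameSettings object, which is neither stored nor saved.
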(event EventBeginPlay
  (Utilities|FlowControl|Sequence
    (:then_0
      ;[1 1 1] Load Audio
      (Class|GameplayStatics|SetBaseSoundMix "/Game/MainMenuSystem/Audio/SM_Master.SM_Master")
      (bind _returnvalue (SaveGame|DoesSaveGameExist "SaveAudio"))
      (if _returnvalue
        (bind _returnvalue_2 (SaveGame|LoadGamefromSlot "SaveAudio"))
        (bind _asbp_save_game_settings (Utilities|Casting|CastToBP_SaveGameSettings _returnvalue_2))
        (Audio|SetSoundMixClassOverride "/Game/MainMenuSystem/Audio/SM_Master.SM_Master" "/Game/MainMenuSystem/Audio/SC_Master.SC_Master" (Variables|/Game/MainMenuSystem/SaveGame/BP_SaveGameSettings.BP_SaveGameSettings_C|GetMasterVolume _asbp_save_game_settings) 1.0 0.0 true)
        (Audio|SetSoundMixClassOverride "/Game/MainMenuSystem/Audio/SM_Music.SM_Music" "/Game/MainMenuSystem/Audio/SC_Music.SC_Music" (Variables|/Game/MainMenuSystem/SaveGame/BP_SaveGameSettings.BP_SaveGameSettings_C|GetMusicVolume _asbp_save_game_settings) 1.0 0.0 true)
        (Audio|SetSoundMixClassOverride "/Game/MainMenuSystem/Audio/SM_SFX.SM_SFX" "/Game/MainMenuSystem/Audio/SC_SFX.SC_SFX" (Variables|/Game/MainMenuSystem/SaveGame/BP_SaveGameSettings.BP_SaveGameSettings_C|GetSFXVolume _asbp_save_game_settings) 1.0 0.0 true)
        (Audio|SetSoundMixClassOverride "/Game/MainMenuSystem/Audio/SM_Voice.SM_Voice" "/Game/MainMenuSystem/Audio/SC_Voice.SC_Voice" (Variables|/Game/MainMenuSystem/SaveGame/BP_SaveGameSettings.BP_SaveGameSettings_C|GetVoiceVolume _asbp_save_game_settings) 1.0 0.0 true)
        (else
          (SaveGame|CreateSaveGameObject "/Game/MainMenuSystem/SaveGame/BP_SaveGameSettings.BP_SaveGameSettings_C"))))
    (:then_1
      ;[1 1 1] Load Mouse Settings
      (bind _returnvalue_3 (SaveGame|DoesSaveGameExist "SaveMouseSettings"))
      (if _returnvalue_3
        (bind _returnvalue_4 (SaveGame|LoadGamefromSlot "SaveMouseSettings"))
        (bind _asbp_save_game_settings_2 (Utilities|Casting|CastToBP_SaveGameSettings _returnvalue_4))
        (bind _asbp_third_person_character (Utilities|Casting|CastToBP_ThirdPersonCharacter (Game|GetPlayerCharacter 0)))
        (Variables|/Game/MainMenuSystem/Blueprints/ThirdPerson/BP_ThirdPersonCharacter.BP_ThirdPersonCharacter_C|SetMouseSensitivity _asbp_third_person_character (Variables|/Game/MainMenuSystem/SaveGame/BP_SaveGameSettings.BP_SaveGameSettings_C|GetMouseSensitivity _asbp_save_game_settings_2))
        (Variables|/Game/MainMenuSystem/Blueprints/ThirdPerson/BP_ThirdPersonCharacter.BP_ThirdPersonCharacter_C|SetInvertValue _asbp_third_person_character (Variables|/Game/MainMenuSystem/SaveGame/BP_SaveGameSettings.BP_SaveGameSettings_C|GetInvertValue _asbp_save_game_settings_2))
        (else
          (SaveGame|CreateSaveGameObject "/Game/MainMenuSystem/SaveGame/BP_SaveGameSettings.BP_SaveGameSettings_C"))))))

(fn ConstructionScript)