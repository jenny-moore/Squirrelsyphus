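; Boulder hazard that drops when triggered and knocks away what it overlaps.
; OnTrigger reveals the rock, enables gravity and plays audio, then after Lifetime asks the Trigger stored by TriggerCallback for a replacement and destroys itself.
; Overlaps use scaled rock velocity to push a chain's EndAcorn or launch the third-person character, playing Collision.
; OnReset restores the starting transform, hides the rock, and disables its physics and collision.
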(event EventBeginPlay
  (Variables|Default|SetInitialTransform (Transformation|GetActorTransform)))

(event EventOnReset
  (Physics|SetSimulatePhysics (Variables|Default|GetRock) false)
  (Collision|SetCollisionEnabled (Variables|Default|GetRock) "NoCollision")
  (Transformation|SetActorTransform (Variables|Default|GetInitialTransform))
  (Development|SetHiddeninGame (Variables|Default|GetRock) true false)
  (Variables|Default|Setspawned false)
  (Development|PrintString "Reset"))

(event Collision|EventActorBeginOverlap
  (params (OtherActor :type Actor%20Object%20Reference))
  (bind _rock (Variables|Default|GetRock))
  (bind _returnvalue (Transformation|GetComponentVelocity _rock))
  (bind _returnvalue_2 (* _returnvalue 1e+03))
  (Development|PrintString (Utilities|GetDisplayName OtherActor))
  (bind _asnew_chain_blueprint (Utilities|Casting|CastToNewChain_Blueprint OtherActor)
    (:then
      (Development|PrintString (Utilities|GetObjectName (Variables|/Game/LevelPrototyping/Chain/NewChain_Blueprint.NewChain_Blueprint_C|GetEndAcorn _asnew_chain_blueprint)))
      (Physics|AddForce (Variables|/Game/LevelPrototyping/Chain/NewChain_Blueprint.NewChain_Blueprint_C|GetEndAcorn _asnew_chain_blueprint) _returnvalue_2 "None" true))
    (:CastFailed
      (Development|PrintText "Not Egg!")
      (bind _asbp_third_person_character_exported_2 (Utilities|Casting|CastToBP_ThirdPersonCharacterExported2 OtherActor))
      (Character|LaunchCharacter _asbp_third_person_character_exported_2 _returnvalue_2 true false)))
  (Audio|Components|Audio|Play (Variables|Default|Getcollision) 0.0))

(event EventOnTrigger
  (params (targetTransform :type Transform) (Player :type Actor%20Object%20Reference))
  (if (not (Variables|Default|Getspawned))
    (Development|PrintString "Enabled Gravity")
    (Rendering|SetActorHiddenInGame false)
    (Physics|SetEnableGravity (Variables|Default|GetRock) true)
    (bind _output_get (Variables|Default|Setspawned true))
    (Development|PrintString (Utilities|String|ToString(Boolean) _output_get))
    (Audio|Components|Audio|Play (Variables|Default|GetAudio) 0.0)
    (Utilities|FlowControl|Delay (Variables|Default|GetLifetime))
    (Audio|Components|Audio|Stop (Variables|Default|GetAudio))
    (Rendering|SetActorHiddenInGame true)
    (Default|MakeNewBoulder (Variables|Default|GetTrigger))
    (Development|PrintString "Rock Gone")
    (Actor|DestroyActor)))

(fn ConstructionScript)

(fn TriggerCallback
  (params (BoulderTrigger :type BP%20Boulder%20Trigger%20Object%20Reference))
  (Variables|Default|SetTrigger BoulderTrigger))