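; BP_BirdTrigger is an obstacle trigger that sets off a linked BP_Bird when the player character enters its box.
; At BeginPlay it caches the bird's starting transform.
; The first player overlap latches Triggered, then passes the bird a reference to the trigger plus the player and their current transform.
; MakeNewBird, not called within this Blueprint, spawns a replacement at the cached transform and re-arms the trigger.
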(event OnComponentBeginOverlap(Box)
  (params (OverlappedComponent :type Primitive%20Component%20Object%20Reference) (OtherActor :type Actor%20Object%20Reference) (OtherComp :type Primitive%20Component%20Object%20Reference) (OtherBodyIndex :type Integer) (bFromSweep :type Boolean) (SweepResult :type Hit%20Result%20Structure%20%28by%20ref%29))
  (bind _spawnedbird (Variables|Default|GetSpawnedBird))
  (if (not (Variables|Default|Gettriggered))
    (bind _asbp_third_person_character_exported_2 (Utilities|Casting|CastToBP_ThirdPersonCharacterExported2 OtherActor))
    (Variables|Default|Settriggered true)
    (Default|TriggerCallback _spawnedbird self)
    (Class|BPIObstacles|OnTrigger(Message) _spawnedbird (Transformation|GetActorTransform _asbp_third_person_character_exported_2) _asbp_third_person_character_exported_2)))

(event EventBeginPlay
  (CallFunction|SetInitialTransform))

(fn ConstructionScript)

(fn SetInitialTransform
  (Variables|Default|SetInitialBirdTransform (Transformation|GetWorldTransform (Variables|/Script/Engine.Actor|GetRootComponent (Variables|Default|GetSpawnedBird)))))

(fn MakeNewBird
  (params (InitialTransform :type Boolean))
  (bind _initialbirdtransform (Variables|Default|GetInitialBirdTransform))
  (bind _returnvalue (Game|SpawnActorfromClass "/Game/Obstacles/BP_Bird.BP_Bird_C" _initialbirdtransform "Undefined" "MultiplyWithRoot" 0 0))
  (Variables|/Game/Obstacles/BP_Bird.BP_Bird_C|SetInitial%20Transform _returnvalue _initialbirdtransform)
  (Variables|Default|SetSpawnedBird _returnvalue)
  (Variables|Default|Settriggered false))