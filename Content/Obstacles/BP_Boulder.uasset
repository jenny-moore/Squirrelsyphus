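; BP_Boulder is a falling boulder obstacle that knocks back whatever it hits.
; When triggered, it appears with gravity and sound, then after its lifetime asks its registered trigger for a replacement and destroys itself.
; Overlaps and rock hits launch the player character, or push a chain's end acorn, using rock velocity plus an offset, scaled by launch force.
; A reset event disables physics and collision, restores the initial transform and hides the rock.
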(event OnComponentHit(Rock)
  (params (HitComponent :type Primitive%20Component%20Object%20Reference) (OtherActor :type Actor%20Object%20Reference) (OtherComp :type Primitive%20Component%20Object%20Reference) (NormalImpulse :type Vector :default "0, 0, 0") (Hit :type Hit%20Result%20Structure%20%28by%20ref%29))
  (bind _launchforce (Variables|Default|GetLaunchForce))
  (bind _launchoffset (Variables|Default|GetLaunchOffset))
  (bind _rock (Variables|Default|GetRock))
  (bind _returnvalue (Transformation|GetComponentVelocity _rock))
  (bind _returnvalue_2 (+ _returnvalue _launchoffset))
  (bind _returnvalue_3 (* _returnvalue_2 _launchforce))
  (bind _returnvalue_4 (* _returnvalue_3 25.0))
  (bind _asnew_chain_blueprint (Utilities|Casting|CastToNewChain_Blueprint OtherActor)
    (:then
      (Development|PrintString (Utilities|GetDisplayName (Variables|/Game/LevelPrototyping/Chain/NewChain_Blueprint.NewChain_Blueprint_C|GetEndAcorn _asnew_chain_blueprint)))
      (Development|PrintString (Utilities|String|ToString(Vector) _returnvalue_4))
      (Physics|AddForce (Variables|/Game/LevelPrototyping/Chain/NewChain_Blueprint.NewChain_Blueprint_C|GetEndAcorn _asnew_chain_blueprint) _returnvalue_4 "None" true))
    (:CastFailed
      (bind _asbp_third_person_character_exported_2 (Utilities|Casting|CastToBP_ThirdPersonCharacterExported2 OtherActor))
      (Development|PrintString "HIT PLAYER!")
      (Character|LaunchCharacter _asbp_third_person_character_exported_2 _returnvalue_3 true true)))
  (Audio|Components|Audio|Play (Variables|Default|Getcollision) 0.0))

(event EventBeginPlay
  (Variables|Default|SetInitialTransform (Transformation|GetActorTransform)))

(event EventOnReset
  (Physics|SetSimulatePhysics (Variables|Default|GetRock) false)
  (Collision|SetCollisionEnabled (Variables|Default|GetRock) "NoCollision")
  (Transformation|SetActorTransform (Variables|Default|GetInitialTransform))
  (Development|SetHiddeninGame (Variables|Default|GetRock) true false)
  (Variables|Default|Setspawned false))

(event Collision|EventActorBeginOverlap
  (params (OtherActor :type Actor%20Object%20Reference))
  (bind _launchforce (Variables|Default|GetLaunchForce))
  (bind _launchoffset (Variables|Default|GetLaunchOffset))
  (bind _rock (Variables|Default|GetRock))
  (bind _returnvalue (Transformation|GetComponentVelocity _rock))
  (bind _returnvalue_2 (+ _returnvalue _launchoffset))
  (bind _returnvalue_3 (* _returnvalue_2 _launchforce))
  (bind _returnvalue_4 (* _returnvalue_3 25.0))
  (bind _asnew_chain_blueprint (Utilities|Casting|CastToNewChain_Blueprint (stale OnComponentHit(Rock) OtherActor))
    (:then
      (Development|PrintString (Utilities|GetDisplayName (Variables|/Game/LevelPrototyping/Chain/NewChain_Blueprint.NewChain_Blueprint_C|GetEndAcorn _asnew_chain_blueprint)))
      (Development|PrintString (Utilities|String|ToString(Vector) _returnvalue_4))
      (Physics|AddForce (Variables|/Game/LevelPrototyping/Chain/NewChain_Blueprint.NewChain_Blueprint_C|GetEndAcorn _asnew_chain_blueprint) _returnvalue_4 "None" true))
    (:CastFailed
      (bind _asbp_third_person_character_exported_2 (Utilities|Casting|CastToBP_ThirdPersonCharacterExported2 (stale OnComponentHit(Rock) OtherActor)))
      (Development|PrintString "HIT PLAYER!")
      (Character|LaunchCharacter _asbp_third_person_character_exported_2 _returnvalue_3 true true)))
  (Audio|Components|Audio|Play (Variables|Default|Getcollision) 0.0))

(event EventOnTrigger
  (params (targetTransform :type Transform) (Player :type Actor%20Object%20Reference))
  (if (not (Variables|Default|Getspawned))
    (Rendering|SetActorHiddenInGame false)
    (Physics|SetEnableGravity (Variables|Default|GetRock) true)
    (Variables|Default|Setspawned true)
    (Audio|Components|Audio|Play (Variables|Default|GetAudio) 0.0)
    (Utilities|FlowControl|Delay (Variables|Default|GetLifetime))
    (Audio|Components|Audio|Stop (Variables|Default|GetAudio))
    (Rendering|SetActorHiddenInGame true)
    (Default|MakeNewBoulder (Variables|Default|GetTrigger) (Variables|Default|GetLaunchForce))
    (Actor|DestroyActor)))

(fn ConstructionScript)

(fn TriggerCallback
  (params (BoulderTrigger :type BP%20Boulder%20Trigger%20Object%20Reference))
  (Variables|Default|SetTrigger BoulderTrigger))