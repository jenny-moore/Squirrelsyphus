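; Geyser obstacle that periodically blows steam and flings player characters and chain objects upward while pulling them toward its center.
; Activate starts an offset, interval-driven loop calling TriggerBlow, which starts steam and, unless audio is already playing, sound plus looping timers for force and blow duration.
; ForceCollider overlaps maintain the target list; GeyserLift launches characters or adds a velocity-change impulse to the chain's EndAcorn.
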(event OnComponentBeginOverlap(forceCollider)
  (params (OverlappedComponent :type Primitive%20Component%20Object%20Reference) (OtherActor :type Actor%20Object%20Reference) (OtherComp :type Primitive%20Component%20Object%20Reference) (OtherBodyIndex :type Integer) (bFromSweep :type Boolean) (SweepResult :type Hit%20Result%20Structure%20%28by%20ref%29))
  (bind _validtargets (Variables|Default|GetvalidTargets))
  (bind _asbp_third_person_character_exported_2 (Utilities|Casting|CastToBP_ThirdPersonCharacterExported2 OtherActor)
    (:then
      (Utilities|Array|AddUnique _validtargets _asbp_third_person_character_exported_2))
    (:CastFailed
      (bind _asnew_chain_blueprint (Utilities|Casting|CastToNewChain_Blueprint OtherActor))
      (Utilities|Array|AddUnique _validtargets _asnew_chain_blueprint))))

(event OnComponentEndOverlap(forceCollider)
  (params (OverlappedComponent :type Primitive%20Component%20Object%20Reference) (OtherActor :type Actor%20Object%20Reference) (OtherComp :type Primitive%20Component%20Object%20Reference) (OtherBodyIndex :type Integer))
  (Utilities|Array|RemoveItem (Variables|Default|GetvalidTargets) OtherActor))

(event Custom|GeyserCycle
  (params (blowTime :type Float%20%28double-precision%29) (Offset :type Float%20%28double-precision%29) (interval :type Float%20%28double-precision%29))
  (Utilities|FlowControl|Delay Offset)
  (CallFunction|TriggerBlow blowTime :!label _label)
  (Utilities|FlowControl|Delay interval)
  (if (Variables|Default|GetisActive)
    (goto _label)))

(event Custom|ApplyGeyserForce
  (if (Variables|Default|GetisActive)
    (for _array_element (Variables|Default|GetvalidTargets)
      (CallFunction|GeyserLift _array_element))))

(event Custom|StopGeyser
  (Utilities|Time|ClearandInvalidateTimerbyHandle (Variables|Default|GetforceTimerHandle))
  (Components|Activation|Deactivate (Variables|Default|Getsteam)))

(fn ConstructionScript)

(fn TriggerBlow
  (params (interval :type Float%20%28double-precision%29))
  (Variables|Default|SetisActive true)
  (Components|Activation|Activate (Variables|Default|Getsteam) false)
  (if (not (Audio|Components|Audio|IsPlaying (Variables|Default|GetAudio)))
    (Audio|Components|Audio|Play (Variables|Default|GetAudio) 0.0)
    (bind _returnvalue (Utilities|Time|SetTimerbyEvent (EventDispatchers|CreateEvent :!event Custom|ApplyGeyserForce) 0.1 true true))
    (Variables|Default|SetforceTimerHandle _returnvalue)
    (Utilities|Time|SetTimerbyEvent (EventDispatchers|CreateEvent :!event Custom|StopGeyser) interval true)))

(fn GeyserLift
  (params (target :type Actor%20Object%20Reference))
  (bind _returnvalue (Transformation|GetActorTransform target))
  (bind _forcecollider (Variables|Default|GetforceCollider))
  (bind _geyserforce (Variables|Default|GetgeyserForce))
  (bind _location (Math|Transform|BreakTransform _returnvalue))
  (bind _returnvalue_2 (Transformation|GetWorldLocation _forcecollider))
  (bind _returnvalue_3 (- _returnvalue_2 _location))
  (bind (_x _y) (Math|Vector|BreakVector _returnvalue_3))
  (bind _returnvalue_4 (Math|Vector|MakeVector _x _y _geyserforce))
  (bind _asbp_third_person_character_exported_2 (Utilities|Casting|CastToBP_ThirdPersonCharacterExported2 target)
    (:then
      (Character|LaunchCharacter _asbp_third_person_character_exported_2 _returnvalue_4 false false))
    (:CastFailed
      (bind _asnew_chain_blueprint (Utilities|Casting|CastToNewChain_Blueprint target))
      (Physics|AddImpulse (Variables|/Game/LevelPrototyping/Chain/NewChain_Blueprint.NewChain_Blueprint_C|GetEndAcorn _asnew_chain_blueprint) _returnvalue_4 "None" true))))

(fn Activate
  (params (blowTime :type Float%20%28double-precision%29) (interval :type Float%20%28double-precision%29) (Offset :type Float%20%28double-precision%29))
  (CallFunction|GeyserCycle blowTime Offset interval))