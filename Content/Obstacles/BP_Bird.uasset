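; Bird obstacle that, once triggered, dive-bombs the player and knocks them away.
; Tick moves it at fixed speed per frame toward the player, locking a point just below them once within range.
; Box overlap launches the character, or pushes a chain's end acorn, with a sound.
; After reaching its target or striking the character, it returns to its start, calls MakeNewBird on its trigger and destroys itself.
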(event OnComponentBeginOverlap(Box)
  (params (OverlappedComponent :type Primitive%20Component%20Object%20Reference) (OtherActor :type Actor%20Object%20Reference) (OtherComp :type Primitive%20Component%20Object%20Reference) (OtherBodyIndex :type Integer) (bFromSweep :type Boolean) (SweepResult :type Hit%20Result%20Structure%20%28by%20ref%29))
  (bind _returnvalue (Transformation|GetActorRotation))
  (bind _launchspeed (Variables|Default|GetLaunchSpeed))
  (bind _returnvalue_2 (Math|Rotator|GetRotationXVector _returnvalue))
  (bind (_x _y) (Math|Vector|BreakVector _returnvalue_2))
  (bind _returnvalue_3 (Math|Vector|MakeVector _x _y 0.3))
  (bind _returnvalue_4 (* _returnvalue_3 _launchspeed))
  (bind _asbp_third_person_character_exported_2 (Utilities|Casting|CastToBP_ThirdPersonCharacterExported2 OtherActor)
    (:then
      (Character|LaunchCharacter _asbp_third_person_character_exported_2 _returnvalue_4 true false)
      (Variables|Default|SetmissionActive false))
    (:CastFailed
      (bind _asnew_chain_blueprint (Utilities|Casting|CastToNewChain_Blueprint OtherActor))
      (Physics|AddForce (Variables|/Game/LevelPrototyping/Chain/NewChain_Blueprint.NewChain_Blueprint_C|GetEndAcorn _asnew_chain_blueprint) _returnvalue_4 "None" true)))
  (Audio|Components|Audio|Play (Variables|Default|GetCOLLISIONaudio) 0.0))

(event EventBeginPlay
  (Variables|Default|SetInitial%20Transform (Transformation|GetActorTransform)))

(event EventTick
  (params (DeltaSeconds :type Float%20%28single-precision%29))
  (bind _flightspeed (Variables|Default|GetFlightSpeed))
  (bind _targetplayer (Variables|Default|GettargetPlayer))
  (bind _targetplayer_2 (Variables|Default|GettargetPlayer))
  (bind _returnvalue (Transformation|GetActorLocation _targetplayer_2))
  (bind (_x _y _z) (Math|Vector|BreakVector _returnvalue))
  (if (Utilities|IsValid (Variables|Default|GettargetPlayer)) :!label _label
    (if (Variables|Default|GetmissionActive)
      (if (Variables|Default|GetinRadius)
        _
        (elif (<= (Math|Vector|Distance(Vector) (Transformation|GetActorLocation) (Variables|Default|GetbirdTarget)) 1e+03)
          (if (Utilities|IsValid _targetplayer_2)
            (Variables|Default|SetbirdTarget (Math|Vector|MakeVector _x _y (+ _z -1e+02)))
            (Variables|Default|SetinRadius true)
            (else
              (goto _label)))
          (elif (Utilities|IsValid _targetplayer)
            (Variables|Default|SetbirdTarget (Transformation|GetActorLocation _targetplayer))
            (else
              (goto _label)))))
      (else
        (Variables|Default|SetbirdTarget (.Location (Math|Transform|BreakTransform (Variables|Default|GetInitial%20Transform))))))
    (Transformation|SetActorLocation (+ (Transformation|GetActorLocation) (* (Math|Vector|Normalize (- (Variables|Default|GetbirdTarget) (Transformation|GetActorLocation))) (Variables|Default|GetFlightSpeed))) true false)
    (Transformation|SetActorRotation (Math|Rotator|FindLookatRotation (Transformation|GetActorLocation) (Variables|Default|GetbirdTarget)))
    ;[0.15 0.15 0.15 0.5] Is Close Enough to Target to Classify as Hit?
    (Variables|Default|SetError (Math|Vector|Distance(Vector) (Transformation|GetActorLocation) (Variables|Default|GetbirdTarget)))
    (if (<= (Math|Vector|Distance(Vector) (Transformation|GetActorLocation) (Variables|Default|GetbirdTarget)) _flightspeed) :!label _label_2
      (if (Variables|Default|GetmissionActive)
        (Variables|Default|SetmissionActive false)
        (goto _label_2)
        (elif (<= (Math|Vector|Distance(Vector) (Transformation|GetActorLocation) (.Location (Math|Transform|BreakTransform (Variables|Default|GetInitial%20Transform)))) _flightspeed)
          (Default|MakeNewBird (Variables|Default|Gettrigger) false)
          (Actor|DestroyActor))))))

(event EventOnTrigger
  (params (targetTransform :type Transform) (Player :type Actor%20Object%20Reference))
  (bind _flightspeed (Variables|Default|GetFlightSpeed))
  (Utilities|FlowControl|Delay 1.0)
  (Variables|Default|SettargetPlayer Player)
  (if (not (Variables|Default|Getspawned))
    (Rendering|SetActorHiddenInGame false)
    (Audio|Components|Audio|Play (Variables|Default|GetAudio) 0.0)
    (if (Utilities|IsValid (Variables|Default|GettargetPlayer)) :!label _label
      (Variables|Default|SetbirdTarget (Transformation|GetActorLocation (Variables|Default|GettargetPlayer)))
      (Transformation|SetActorLocation (+ (Transformation|GetActorLocation) (* (Math|Vector|Normalize (- (Variables|Default|GetbirdTarget) (Transformation|GetActorLocation))) (Variables|Default|GetFlightSpeed))) true false :!label _label_2)
      (Transformation|SetActorRotation (Math|Rotator|FindLookatRotation (Transformation|GetActorLocation) (Variables|Default|GetbirdTarget)))
      ;[0.15 0.15 0.15 0.5] Is Close Enough to Target to Classify as Hit?
      (Variables|Default|SetError (Math|Vector|Distance(Vector) (Transformation|GetActorLocation) (Variables|Default|GetbirdTarget)))
      (if (<= (Math|Vector|Distance(Vector) (Transformation|GetActorLocation) (Variables|Default|GetbirdTarget)) _flightspeed) :!label _label_3
        (if (Variables|Default|GetmissionActive)
          (Variables|Default|SetmissionActive false)
          (goto _label_3)
          (elif (<= (Math|Vector|Distance(Vector) (Transformation|GetActorLocation) (.Location (Math|Transform|BreakTransform (Variables|Default|GetInitial%20Transform)))) _flightspeed)
            (Default|MakeNewBird (Variables|Default|Gettrigger) false)
            (Actor|DestroyActor))))
      (else
        (if (Utilities|IsValid (Variables|Default|GettargetPlayer)) :!label _label_4
          (if (Variables|Default|GetmissionActive)
            (if (Variables|Default|GetinRadius)
              (goto _label_2)
              (elif (<= (Math|Vector|Distance(Vector) (Transformation|GetActorLocation) (Variables|Default|GetbirdTarget)) 1e+03)
                (if (Utilities|IsValid (Variables|Default|GettargetPlayer))
                  (Variables|Default|SetbirdTarget (Math|Vector|MakeVector (.X (Math|Vector|BreakVector (Transformation|GetActorLocation (Variables|Default|GettargetPlayer)))) (.Y (Math|Vector|BreakVector (Transformation|GetActorLocation (Variables|Default|GettargetPlayer)))) (+ (.Z (Math|Vector|BreakVector (Transformation|GetActorLocation (Variables|Default|GettargetPlayer)))) -1e+02)))
                  (Variables|Default|SetinRadius true)
                  (goto _label_2)
                  (else
                    (goto _label_4)))
                (else
                  (goto _label))))
            (else
              (Variables|Default|SetbirdTarget (.Location (Math|Transform|BreakTransform (Variables|Default|GetInitial%20Transform))))
              (goto _label_2))))))))

(fn ConstructionScript)

(fn DoFlight
  (params (targetTransform :type Transform) (deltaSeconds :type Float%20%28double-precision%29))
  (Transformation|SetActorLocation (+ (.Location (Math|Transform|BreakTransform (Variables|Default|GetInitial%20Transform))) (Math|Vector|Normalize (- (.Location (Math|Transform|BreakTransform targetTransform)) (.Location (Math|Transform|BreakTransform (Variables|Default|GetInitial%20Transform)))))) false false))

(fn TriggerCallback
  (params (BirdTrigger :type BP%20Bird%20Trigger%20Object%20Reference))
  (Variables|Default|Settrigger BirdTrigger))