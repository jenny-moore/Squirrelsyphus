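; BP_Wind is an obstacle that blows intermittent gusts, pushing physics objects inside its WindVolume.
; A Delay on Tick toggles Blowing every ten seconds, with a DoOnce starting the Niagara effect and gust sounds once per cycle.
; Overlap events track actors and components, and each blowing tick applies scaled WindForce to simulating bodies from both lists.
; WindForce also sets the Niagara wind velocity at BeginPlay.
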(event OnComponentBeginOverlap(WindVolume)
  (params (OverlappedComponent :type Primitive%20Component%20Object%20Reference) (OtherActor :type Actor%20Object%20Reference) (OtherComp :type Primitive%20Component%20Object%20Reference) (OtherBodyIndex :type Integer) (bFromSweep :type Boolean) (SweepResult :type Hit%20Result%20Structure%20%28by%20ref%29))
  (Utilities|Array|Add (Variables|Default|GetOverlappingActors) OtherActor)
  (Utilities|Array|Add (Variables|Default|GetOverlappingComponents) OtherComp)
  (Development|PrintString (Utilities|GetObjectName OtherComp)))

(event OnComponentEndOverlap(WindVolume)
  (params (OverlappedComponent :type Primitive%20Component%20Object%20Reference) (OtherActor :type Actor%20Object%20Reference) (OtherComp :type Primitive%20Component%20Object%20Reference) (OtherBodyIndex :type Integer))
  (Utilities|Array|RemoveItem (Variables|Default|GetOverlappingActors) OtherActor)
  (Utilities|Array|RemoveItem (Variables|Default|GetOverlappingComponents) OtherComp))

(event EventBeginPlay
  (Niagara|SetNiagaraVariable(Vector3) (Variables|Default|GetNS_Wind) "WindVelocity" (Variables|Default|GetWindForce)))

(event EventTick
  (params (DeltaSeconds :type Float%20%28single-precision%29))
  (bind _wind_loop (Variables|Default|GetWind_Loop))
  (bind _windforce (Variables|Default|GetWindForce))
  (bind _windstrength (Variables|Default|GetWindStrength))
  (bind _ns_wind (Variables|Default|GetNS_Wind))
  (bind _returnvalue (* _windforce _windstrength))
  (Utilities|FlowControl|Sequence
    (:then_0
      (if (Variables|Default|GetBlowing)
        (Utilities|FlowControl|Sequence
          (:then_0
            (Utilities|FlowControl|DoOnce false :!label _label
              (:Completed
                (Components|Activation|SetActive _ns_wind true false)
                (Audio|Components|Audio|Play (Variables|Default|GetWind_Gust) 0.0)
                (Audio|Components|Audio|Play _wind_loop 2.579125))))
          (:then_1
            (for _array_element (Variables|Default|GetOverlappingActors)
              (if (Physics|IsSimulatingPhysics (Actor|GetComponentbyClass _array_element "/Script/Engine.StaticMeshComponent") "None")
                (Physics|AddForce (Actor|GetComponentbyClass _array_element "/Script/Engine.StaticMeshComponent") _returnvalue "None" false)))
            (for _array_element_2 (Variables|Default|GetOverlappingComponents)
              (if (Physics|IsSimulatingPhysics _array_element_2 "None")
                (Physics|AddForce _array_element_2 _returnvalue "None" false)))))
        (else
          (Components|Activation|SetActive _ns_wind false false)
          (goto _label Reset))))
    (:then_1
      (Utilities|FlowControl|Delay 1e+01)
      (Variables|Default|SetBlowing (not (Variables|Default|GetBlowing)))
      (Audio|Components|Audio|Stop _wind_loop))))

(fn ConstructionScript)