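; Trigger volume for a boulder obstacle, set off when the third-person player character overlaps its box.
; On begin play it records the world transform of the referenced boulder's Rock component.
; On overlap it passes itself to the boulder through TriggerCallback, then calls OnTrigger on it.
; MakeNewBoulder, not called within this Blueprint, spawns a replacement at the saved location and rotation and stores it as the new target.
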(event OnComponentBeginOverlap(Box)
  (params (OverlappedComponent :type Primitive%20Component%20Object%20Reference) (OtherActor :type Actor%20Object%20Reference) (OtherComp :type Primitive%20Component%20Object%20Reference) (OtherBodyIndex :type Integer) (bFromSweep :type Boolean) (SweepResult :type Hit%20Result%20Structure%20%28by%20ref%29))
  (bind _spawnedboulder (Variables|Default|GetSpawnedBoulder))
  (Utilities|Casting|CastToBP_ThirdPersonCharacterExported2 OtherActor)
  (Default|TriggerCallback _spawnedboulder self)
  (Default|OnTrigger _spawnedboulder))

(event EventBeginPlay
  (CallFunction|SetInitialTransform))

(fn ConstructionScript)

(fn MakeNewBoulder
  (bind _initialbouldertransform (Variables|Default|GetInitialBoulderTransform))
  (bind _returnvalue (Game|SpawnActorfromClass "/Game/Obstacles/BP_Boulder.BP_Boulder_C" (Math|Transform|MakeTransform (.location _initialbouldertransform) (.rotation _initialbouldertransform) "1.000000,1.000000,1.000000") "Undefined" "MultiplyWithRoot" 0 0))
  (Variables|Default|SetSpawnedBoulder _returnvalue))

(fn SetInitialTransform
  (Variables|Default|SetInitialBoulderTransform (Transformation|GetWorldTransform (Variables|/Game/Obstacles/BP_Boulder.BP_Boulder_C|GetRock (Variables|Default|GetSpawnedBoulder)))))