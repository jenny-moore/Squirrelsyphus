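; BP_GeyserTrigger is an obstacle trigger that activates a set of geysers when the player character overlaps its Hitbox.
; It loops through the Geysers array, passing BlowTime and Interval to each Activate call with an index-based Offset that staggers them.
; Each index prints to screen, and the Triggered one-shot check is disconnected, so every player overlap activates the geysers again.
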(event OnComponentBeginOverlap(Hitbox)
  (params (OverlappedComponent :type Primitive%20Component%20Object%20Reference) (OtherActor :type Actor%20Object%20Reference) (OtherComp :type Primitive%20Component%20Object%20Reference) (OtherBodyIndex :type Integer) (bFromSweep :type Boolean) (SweepResult :type Hit%20Result%20Structure%20%28by%20ref%29))
  (Utilities|Casting|CastToBP_ThirdPersonCharacterExported2 OtherActor)
  (for (_array_element _array_index) (Variables|Default|Getgeysers)
    (Default|Activate _array_element (Variables|Default|GetblowTime) (Variables|Default|Getinterval) (* _array_index 0.5))
    (Development|PrintString (Utilities|String|ToString(Integer) _array_index))))

(event EventBeginPlay)

(fn ConstructionScript)