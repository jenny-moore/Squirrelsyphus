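; BP_SquirrelsyphusGame is the game's central UI and music manager, with events for the boot, main, options, new/load/save, pause, loading and quit screens.
; Each show event lazily creates and caches its widget, adds it to the viewport and switches to UI-only input.
; Interactive menus set button focus after a short delay for keyboard navigation.
; Pause and resume toggle game pause, cursor and music, while the main menu stops music.
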(event Custom|PlayMusic
  (params (Sound :type Sound%20Base%20Object%20Reference))
  ;[1 1 1 0.5] Play Music
  (bind _returnvalue (Audio|SpawnSound2D Sound 1.0 1.0 0.0 0 true))
  (Variables|Default|SetGameMusic _returnvalue))

(event Custom|Show%20WBP_LoadGame
  (bind _returnvalue (Game|GetPlayerController 0))
  ;[1 1 1] Show WBP_LoadGame
  (Utilities|IsValid (Variables|Widjets|GetLoadGameWBP)
    (:Is%20Valid
      _)
    (:Is%20Not%20Valid
      (bind _returnvalue_2 (UserInterface|CreateWidget "/Game/MainMenuSystem/UI/WBP_LoadGame.WBP_LoadGame_C" _returnvalue))
      (bind _output_get (Variables|Widjets|SetLoadGameWBP _returnvalue_2))))
  (UserInterface|Viewport|AddtoViewport _output_get 0)
  (Input|SetInputModeUIOnly _returnvalue _output_get "DoNotLock" false)
  (Utilities|FlowControl|Delay 0.2)
  (Widget|SetKeyboardFocus (Variables|/Game/MainMenuSystem/UI/WBP_LoadGame.WBP_LoadGame_C|GetBackButton _output_get)))

(event Custom|Show%20WBP_BootScreen
  (bind _returnvalue (Game|GetPlayerController 0))
  ;[1 1 1] Show WBP_BootScreen
  (Utilities|IsValid (Variables|Widjets|GetBootScreenWBP)
    (:Is%20Valid
      _)
    (:Is%20Not%20Valid
      (bind _returnvalue_2 (UserInterface|CreateWidget "/Game/MainMenuSystem/UI/WBP_BootScreen.WBP_BootScreen_C" _returnvalue))
      (bind _output_get (Variables|Widjets|SetBootScreenWBP _returnvalue_2))))
  (UserInterface|Viewport|AddtoViewport _output_get 0)
  (Input|SetInputModeUIOnly _returnvalue (Variables|Widjets|GetBootScreenWBP) "DoNotLock" false)
  (Variables|/Script/Engine.PlayerController|SetbShowMouseCursor _returnvalue false))

(event Custom|Show%20WBP_MainMenu
  (bind _returnvalue (Game|GetPlayerController 0))
  (bind _gamemusic (Variables|Default|GetGameMusic))
  ;[1 1 1] Show WBP_MainMenu
  (Utilities|IsValid (Variables|Widjets|GetMainMenuWBP)
    (:Is%20Valid
      _)
    (:Is%20Not%20Valid
      (bind _returnvalue_2 (UserInterface|CreateWidget "/Game/MainMenuSystem/UI/WBP_MainMenu.WBP_MainMenu_C" _returnvalue))
      (bind _output_get (Variables|Widjets|SetMainMenuWBP _returnvalue_2))))
  (UserInterface|Viewport|AddtoViewport _output_get 0)
  (Input|SetInputModeUIOnly _returnvalue (Variables|Widjets|GetMainMenuWBP) "DoNotLock" false)
  (Utilities|FlowControl|Delay 0.2)
  (Widget|SetKeyboardFocus (Variables|/Game/MainMenuSystem/UI/WBP_MainMenu.WBP_MainMenu_C|GetNewGameButton (Variables|Widjets|GetMainMenuWBP)))
  (Variables|/Script/Engine.PlayerController|SetbShowMouseCursor _returnvalue true)
  (Utilities|IsValid _gamemusic
    (:Is%20Valid
      (Audio|Components|Audio|Stop _gamemusic))))

(event Custom|Show%20WBP_PauseMenu
  (bind _returnvalue (Game|GetPlayerController 0))
  (bind _gamemusic (Variables|Default|GetGameMusic))
  ;[1 1 1] Show WBP_PauseMenu
  (Utilities|IsValid (Variables|Widjets|GetPauseMenuWBP)
    (:Is%20Valid
      _)
    (:Is%20Not%20Valid
      (bind _returnvalue_2 (UserInterface|CreateWidget "/Game/MainMenuSystem/UI/WBP_PauseMenu.WBP_PauseMenu_C" _returnvalue))
      (bind _output_get (Variables|Widjets|SetPauseMenuWBP _returnvalue_2))))
  (UserInterface|Viewport|AddtoViewport _output_get 0)
  (Input|SetInputModeUIOnly _returnvalue (Variables|Widjets|GetPauseMenuWBP) "DoNotLock" false)
  (Utilities|FlowControl|Delay 0.2)
  (Widget|SetKeyboardFocus (Variables|/Game/MainMenuSystem/UI/WBP_PauseMenu.WBP_PauseMenu_C|GetResumeButton (Variables|Widjets|GetPauseMenuWBP)))
  (Game|SetGamePaused true)
  (Variables|/Script/Engine.PlayerController|SetbShowMouseCursor _returnvalue true)
  (Utilities|IsValid _gamemusic
    (:Is%20Valid
      (Class|AudioComponent|SetPaused _gamemusic true))))

(event Custom|Show%20WBP_LoadingScreen
  (bind _returnvalue (Game|GetPlayerController 0))
  ;[1 1 1] Show_WBP_LoadingScreen
  (Utilities|IsValid (Variables|Widjets|GetLoadingScreenWBP)
    (:Is%20Valid
      _)
    (:Is%20Not%20Valid
      (bind _returnvalue_2 (UserInterface|CreateWidget "/Game/MainMenuSystem/UI/WBP_LoadingScreen.WBP_LoadingScreen_C" _returnvalue))
      (bind _output_get (Variables|Widjets|SetLoadingScreenWBP _returnvalue_2))))
  (UserInterface|Viewport|AddtoViewport _output_get 0)
  (Input|SetInputModeUIOnly _returnvalue (Variables|Widjets|GetLoadingScreenWBP) "DoNotLock" false)
  (Variables|/Script/Engine.PlayerController|SetbShowMouseCursor _returnvalue false))

(event Custom|Show%20WBP_QuitGame
  (bind _returnvalue (Game|GetPlayerController 0))
  ;[1 1 1] Show WBP_QuitGame
  (Utilities|IsValid (Variables|Widjets|GetQuitGameWBP)
    (:Is%20Valid
      _)
    (:Is%20Not%20Valid
      (bind _returnvalue_2 (UserInterface|CreateWidget "/Game/MainMenuSystem/UI/WBP_QuitGameQuestion.WBP_QuitGameQuestion_C" _returnvalue))
      (bind _output_get (Variables|Widjets|SetQuitGameWBP _returnvalue_2))))
  (UserInterface|Viewport|AddtoViewport _output_get 0)
  (Input|SetInputModeUIOnly _returnvalue _output_get "DoNotLock" false)
  (Utilities|FlowControl|Delay 0.2)
  (Widget|SetKeyboardFocus (Variables|/Game/MainMenuSystem/UI/WBP_QuitGameQuestion.WBP_QuitGameQuestion_C|GetYesButton _output_get)))

(event Custom|Pause%20Menu%20Resume
  (bind _returnvalue (Game|GetPlayerController 0))
  (bind _gamemusic (Variables|Default|GetGameMusic))
  ;[1 1 1] Pause Menu Resume
  (Widget|RemovefromParent (Variables|Widjets|GetPauseMenuWBP))
  (Game|SetGamePaused false)
  (Input|SetInputModeGameOnly _returnvalue false)
  (Variables|/Script/Engine.PlayerController|SetbShowMouseCursor _returnvalue false)
  (Utilities|IsValid _gamemusic
    (:Is%20Valid
      (Class|AudioComponent|SetPaused _gamemusic false))))

(event Custom|Show%20WBP_OptionsMenu
  (bind _returnvalue (Game|GetPlayerController 0))
  ;[1 1 1] Show WBP_OptionsMenu
  (Utilities|IsValid (Variables|Widjets|GetOptionsMenuWBP)
    (:Is%20Valid
      _)
    (:Is%20Not%20Valid
      (bind _returnvalue_2 (UserInterface|CreateWidget "/Game/MainMenuSystem/UI/Options/WBP_OptionsMenu.WBP_OptionsMenu_C" _returnvalue))
      (bind _output_get (Variables|Widjets|SetOptionsMenuWBP _returnvalue_2))))
  (UserInterface|Viewport|AddtoViewport _output_get 0)
  (Input|SetInputModeUIOnly _returnvalue _output_get "DoNotLock" false)
  (Utilities|FlowControl|Delay 0.2)
  (Widget|SetKeyboardFocus (Variables|/Game/MainMenuSystem/UI/Options/WBP_OptionsMenu.WBP_OptionsMenu_C|GetGeneralButton _output_get)))

(event Custom|Show%20WBP_QuitToMainMenu
  (bind _returnvalue (Game|GetPlayerController 0))
  ;[1 1 1] Show WBP_QuitToMainMenu
  (Utilities|IsValid (Variables|Widjets|GetPauseMenuQuitToMainMenu)
    (:Is%20Valid
      _)
    (:Is%20Not%20Valid
      (bind _returnvalue_2 (UserInterface|CreateWidget "/Game/MainMenuSystem/UI/WBP_QuitToMainMenuQuestion.WBP_QuitToMainMenuQuestion_C" _returnvalue))
      (bind _output_get (Variables|Widjets|SetPauseMenuQuitToMainMenu _returnvalue_2))))
  (UserInterface|Viewport|AddtoViewport _output_get 0)
  (Widget|RemovefromParent (Variables|Widjets|GetPauseMenuWBP))
  (Input|SetInputModeUIOnly _returnvalue _output_get "DoNotLock" false)
  (Utilities|FlowControl|Delay 0.2)
  (Widget|SetKeyboardFocus (Variables|/Game/MainMenuSystem/UI/WBP_QuitToMainMenuQuestion.WBP_QuitToMainMenuQuestion_C|GetYesButton _output_get)))

(event Custom|Show%20WBP_NewGame
  (bind _returnvalue (Game|GetPlayerController 0))
  ;[1 1 1] Show WBP_NewGame
  (Utilities|IsValid (Variables|Widjets|GetNewGameWBP)
    (:Is%20Valid
      _)
    (:Is%20Not%20Valid
      (bind _returnvalue_2 (UserInterface|CreateWidget "/Game/MainMenuSystem/UI/WBP_NewGame.WBP_NewGame_C" _returnvalue))
      (bind _output_get (Variables|Widjets|SetNewGameWBP _returnvalue_2))))
  (UserInterface|Viewport|AddtoViewport _output_get 0)
  (Input|SetInputModeUIOnly _returnvalue _output_get "DoNotLock" false)
  (Utilities|FlowControl|Delay 0.2)
  (Widget|SetKeyboardFocus (Variables|/Game/MainMenuSystem/UI/WBP_NewGame.WBP_NewGame_C|GetStartGameButton _output_get)))

(event Custom|Show%20WBP_SaveGame
  (bind _returnvalue (Game|GetPlayerController 0))
  ;[1 1 1] Show WBP_SaveGame
  (Utilities|IsValid (Variables|Widjets|GetSaveGameWBP)
    (:Is%20Valid
      _)
    (:Is%20Not%20Valid
      (bind _returnvalue_2 (UserInterface|CreateWidget "/Game/MainMenuSystem/UI/WBP_SaveGame.WBP_SaveGame_C" _returnvalue))
      (bind _output_get (Variables|Widjets|SetSaveGameWBP _returnvalue_2))))
  (UserInterface|Viewport|AddtoViewport _output_get 0)
  (Input|SetInputModeUIOnly _returnvalue _output_get "DoNotLock" false)
  (Utilities|FlowControl|Delay 0.2)
  (Widget|SetKeyboardFocus (Variables|/Game/MainMenuSystem/UI/WBP_SaveGame.WBP_SaveGame_C|GetBackButton _output_get)))